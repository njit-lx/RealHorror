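; Player camera manager for the horror game that gives BP_Player a smoothed, lagging first-person look with a narrow fixed FOV.
; BeginPlay clamps view pitch, and Tick interpolates a stored rotation from the current camera rotation toward the horror player controller's control rotation.
; The BlueprintUpdateCamera override combines that rotation with the player's camera component location, applying only when the view target is BP_Player.
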(event EventBeginPlay
  (Variables|Default|SetViewPitchMin -75.0)
  (Variables|Default|SetViewPitchMax 75.0))

(event Collision|EventActorBeginOverlap
  (params (OtherActor :type Actor%20Object%20Reference)))

(event EventTick
  (params (DeltaSeconds :type Float%20%28single-precision%29))
  (CallFunction|UpdateTargetRotation))

(fn ConstructionScript)

(fn UpdateTargetRotation
  (Variables|Default|SetRotation (Math|Interpolation|RInterpTo (Camera|GetCameraRotation) (Pawn|GetControlRotation (Class|HorrorBlueprintFunctionLibrary|GetHorrorPlayerController) :!class /Script/Engine.Controller) (Utilities|Time|GetWorldDeltaSeconds) 15.0)))

(fn BlueprintUpdateCamera
  (params (CameraTarget :type Actor%20Object%20Reference))
  (bind _asbp_player (Utilities|Casting|CastToBP_Player CameraTarget))
  (return (Transformation|GetWorldLocation (Variables|/Game/RealHorror/Blueprint/BP_Player.BP_Player_C|GetCamera _asbp_player)) (Variables|Default|GetRotation) 45.0 true))